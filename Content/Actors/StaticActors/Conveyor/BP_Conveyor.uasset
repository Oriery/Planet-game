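; BP_Conveyor is a conveyor actor placed on a planet's surface, with an optional mirrored twin on the opposite side.
; Its construction script orients it radially from the first ActorPlanet found and snaps it to DistanceFromCentreOfPlanet.
; It then mirrors location, rotation and Y-flipped scale onto MyOppositePair through the world origin, and copies OrderOfConveyor to it.
; The event graph holds no active logic.
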(fn `UserConstructionScript`
  (bind _my_opposite_pair (`self.my_opposite_pair`))
  (bind _outactors (`GameplayStatics.GetAllActorsOfClass` "/Script/Planet_Strat.ActorPlanet"))
  (bind _returnvalue (`self.K2_GetActorLocation` (`|GetArrayItem` _outactors)))
  (bind _returnvalue_2 (- (`self.K2_GetActorLocation`) _returnvalue))
  (`self.K2_SetActorRotation` (`KismetMathLibrary.MakeRotFromZX` _returnvalue_2 (`self.GetActorForwardVector`)))
  (`self.K2_SetActorLocation` (+ _returnvalue (* (`KismetMathLibrary.Normal` _returnvalue_2) (`self.DistanceFromCentreOfPlanet`))))
  (if (`KismetSystemLibrary.IsValid` _my_opposite_pair)
    (`self.K2_SetActorLocation` _my_opposite_pair (* (`self.K2_GetActorLocation`) -1.0) false false)
    (`self.K2_SetActorRotation` _my_opposite_pair (`KismetMathLibrary.MakeRotFromZX` (* (`self.GetActorUpVector`) -1.0) (* (`self.GetActorForwardVector`) -1.0)) false)
    (`self.SetActorScale3D` _my_opposite_pair (`KismetMathLibrary.MakeVector` (.x (`self.GetActorScale3D`)) (* -1 (.y (`self.GetActorScale3D`))) (.z (`self.GetActorScale3D`))))
    (bind _asbp_conveyor (cast `/Game/Actors/StaticActors/Conveyor/BP_Conveyor` (`self.my_opposite_pair`)))
    (set `Conveyor.orderOfConveyor` (`self.orderOfConveyor`) _asbp_conveyor)))