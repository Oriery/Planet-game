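; BP_MyHome is a home actor that keeps a linked actor, MyOppositePair, as its point-mirrored counterpart across the world origin.
; Its construction script negates its location for the pair and builds the pair's rotation from inverted up and forward vectors.
; Negating the pair's Y scale completes the inversion, which rotation alone cannot produce.
; The event graph holds no logic.
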(fn `UserConstructionScript`
  (bind _my_opposite_pair (`self.my_opposite_pair`))
  (if (`KismetSystemLibrary.IsValid` _my_opposite_pair)
    (`self.K2_SetActorLocation` _my_opposite_pair (* (`self.K2_GetActorLocation`) -1.0) false false)
    (`self.K2_SetActorRotation` _my_opposite_pair (`KismetMathLibrary.MakeRotFromZX` (* (`self.GetActorUpVector`) -1.0) (* (`self.GetActorForwardVector`) -1.0)) false)
    (`self.SetActorScale3D` _my_opposite_pair (`KismetMathLibrary.MakeVector` (.x (`self.GetActorScale3D`)) (* -1 (.y (`self.GetActorScale3D`))) (.z (`self.GetActorScale3D`))))))