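; Player start for planet levels that snaps itself onto a sphere around the first ActorPlanet found.
; Its construction script points local Z away from the planet center, keeps forward as close as possible, and projects the location to a fixed distance from that center.
; If an opposite pair is assigned, it moves that actor to the point mirrored through the world origin, with up and forward vectors reversed.
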(fn `UserConstructionScript`
  (bind _my_opposite_pair (`self.my_opposite_pair`))
  (bind _outactors (`GameplayStatics.GetAllActorsOfClass` "/Script/Planet_Strat.ActorPlanet"))
  (bind _returnvalue (`self.K2_GetActorLocation` (`|GetArrayItem` _outactors)))
  (bind _returnvalue_2 (- (`self.K2_GetActorLocation`) _returnvalue))
  (`self.K2_SetActorRotation` (`KismetMathLibrary.MakeRotFromZX` _returnvalue_2 (`self.GetActorForwardVector`)))
  (`self.K2_SetActorLocation` (+ _returnvalue (* (`KismetMathLibrary.Normal` _returnvalue_2) 1202.0)))
  (if (`KismetSystemLibrary.IsValid` _my_opposite_pair)
    (`self.K2_SetActorLocation` _my_opposite_pair (* (`self.K2_GetActorLocation`) -1.0) false false)
    (`self.K2_SetActorRotation` _my_opposite_pair (`KismetMathLibrary.MakeRotFromZX` (* (`self.GetActorUpVector`) -1.0) (* (`self.GetActorForwardVector`) -1.0)) false)))