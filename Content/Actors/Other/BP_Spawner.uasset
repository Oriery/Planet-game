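; BP_Spawner is a placeable spawner actor that keeps a linked opposite actor mirrored through the world origin.
; Its construction script moves a valid MyOppositePair to the negated location of this actor.
; It also rotates the pair by negating pitch and offsetting roll and yaw by half a turn, reversing forward and up.
; The event graph holds only disabled stubs, so no spawning logic appears here.
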(fn `UserConstructionScript`
  (bind _my_opposite_pair (`self.my_opposite_pair`))
  (if (`KismetSystemLibrary.IsValid` _my_opposite_pair)
    (`self.K2_SetActorLocation` _my_opposite_pair (* (`self.K2_GetActorLocation`) -1.0) false false)
    (`self.K2_SetActorRotation` _my_opposite_pair (`KismetMathLibrary.MakeRotator` (+ (.roll (`self.K2_GetActorRotation`)) 180.0) (* -1 (.pitch (`self.K2_GetActorRotation`))) (+ (.yaw (`self.K2_GetActorRotation`)) 180.0)) false)))