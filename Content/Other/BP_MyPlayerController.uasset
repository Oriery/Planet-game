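; Player controller that owns the in-game GUI and toggles the in-game main menu.
; On BeginPlay, only the non-authority (remote) side creates the GUI widget and adds it to the viewport.
; Escape drives a FlipFlop that swaps the GUI's widget switcher between the main menu and its default box, switching input mode and cursor visibility to match.
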(event `self.ReceiveBeginPlay`
  (`/Engine/EditorBlueprintResources/ActorMacros.Switch Has Authority`
    (:`Remote`
      (bind _returnvalue (`|CreateWidget` "/Game/GUI/W_InGame_GUI.W_InGame_GUI_C" self))
      (bind _output_get (set `self.W_IngameGUI` _returnvalue))
      (`UserWidget.AddToViewport` _output_get 0))))

(event `Key|Escape`
  (params (Key :type "Key Structure"))
  (bind _w_ingamegui (`self.W_IngameGUI`))
  (bind _widgetswitcher_240 (`/Game/GUI/W_InGame_GUI.WidgetSwitcher_240` _w_ingamegui))
  (:`Pressed`
    (`/Engine/EditorBlueprintResources/StandardMacros.FlipFlop`
      (:`A`
        (`WidgetSwitcher.SetActiveWidget` _widgetswitcher_240 (`/Game/GUI/W_InGame_GUI.W_IngameMainMenu` _w_ingamegui))
        (`WidgetBlueprintLibrary.SetInputMode_GameAndUIEx` self (`self.W_IngameGUI`) "LockAlways" false)
        (set `self.bShowMouseCursor` true))
      (:`B`
        (`WidgetSwitcher.SetActiveWidget` _widgetswitcher_240 (`/Game/GUI/W_InGame_GUI.SizeBox_0` _w_ingamegui))
        (`WidgetBlueprintLibrary.SetInputMode_GameOnly` self)
        (set `self.bShowMouseCursor` false)))))

(fn `UserConstructionScript`)